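; BP_CollideMovingPlacform is a moving platform that the player triggers by entering its sphere trigger.
; Overlap by BP_ThirdPersonCharacter destroys the sphere, making it one-shot, sets IsMoving and waits three seconds.
; The Platform timeline then drives the actor's position as an offset from the location saved at BeginPlay, without sweeping.
; PointA and MoveDuration logic is disconnected, and the custom event functions are empty.
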(event `self.ReceiveBeginPlay`
  ;[1 1 1] Set play and position
  (set `self.start location` (`self.K2_GetActorLocation`)))

(event `Activate plat`
  ;[1 1 1] Process
  (set `self.IsMoving` true)
  (`ActorComponent.K2_DestroyComponent` (`self.Sphere`))
  (`KismetSystemLibrary.Delay` 3.0)
  (bind (_direction _newtrack_2 _newtrack_3) (`Timeline|Platform` :!via `PlayFromStart`)
    (:`Update`
      (`self.K2_SetActorLocation` (+ (`self.start location`) _newtrack_3)))))

(event `self.Sphere.OnComponentBeginOverlap`
  (params (OverlappedComponent :type "PrimitiveComponent Object Reference") (OtherActor :type "Actor Object Reference") (OtherComp :type "PrimitiveComponent Object Reference") (OtherBodyIndex :type Integer) (bFromSweep :type Boolean) (SweepResult :type "HitResult Structure (by ref)"))
  ;[1 1 1] Activate depending on collision
  (cast `/Game/ThirdPerson/Blueprints/BP_ThirdPersonCharacter` OtherActor)
  (`self.Activate plat`))

(fn `CustomEvent`)

(fn `CustomEvent_1`)

(fn `UserConstructionScript`)