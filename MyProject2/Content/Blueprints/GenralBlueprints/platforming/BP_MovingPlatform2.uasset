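; BP_MovingPlatform2 is a moving platform that starts when the player character overlaps its trigger sphere.
; Activation disables the sphere, waits briefly, then plays a timeline that offsets the actor from its BeginPlay location.
; Each timeline update polls player health; on death it stops, snaps the platform home and re-arms the sphere, otherwise the trigger stays disabled.
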(event `self.ReceiveBeginPlay`
  ;[1 1 1] Set play and position
  (set `self.start location` (`self.K2_GetActorLocation`)))

(event `Activate plat`
  (bind _start_location (`self.start location`))
  ;[1 1 1] Process
  (set `self.IsMoving` true)
  (`PrimitiveComponent.SetCollisionEnabled` (`self.Sphere`) "NoCollision")
  (`KismetSystemLibrary.Delay` 5.0)
  (bind (_direction _newtrack_2 _newtrack_3 _newtrack_0) (`Timeline|Platform` :!via `PlayFromStart` :!label _label)
    (:`Update`
      (`self.K2_SetActorLocation` (+ _start_location _newtrack_0))
      ;[1 1 1] If player dies
      (bind _asbp_third_person_character (cast `/Game/ThirdPerson/Blueprints/BP_ThirdPersonCharacter` (`GameplayStatics.GetPlayerCharacter` 0)))
      (if (<= (`/Game/ThirdPerson/Blueprints/BP_ThirdPersonCharacter.health` _asbp_third_person_character) 0.0)
        (`self.K2_SetActorLocation` _start_location)
        (`PrimitiveComponent.SetCollisionEnabled` (`self.Sphere`) "QueryAndPhysics")
        (goto _label :!via `Stop`)))))

(event `self.Sphere.OnComponentBeginOverlap`
  (params (OverlappedComponent :type "PrimitiveComponent Object Reference") (OtherActor :type "Actor Object Reference") (OtherComp :type "PrimitiveComponent Object Reference") (OtherBodyIndex :type Integer) (bFromSweep :type Boolean) (SweepResult :type "HitResult Structure (by ref)"))
  ;[1 1 1] Activate depending on collision
  (cast `/Game/ThirdPerson/Blueprints/BP_ThirdPersonCharacter` OtherActor)
  (`self.Activate plat`))

(fn `CustomEvent`)

(fn `CustomEvent_1`)

(fn `UserConstructionScript`)