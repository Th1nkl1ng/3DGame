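; BP_AIT_Objective is an enemy that counts toward an eliminate-all-enemies objective.
; On BeginPlay it increments EnemiesLeft in BP_ThirdPersonGameMode, and AnyDamage subtracts from AIHealth.
; At zero health it turns on mesh physics, then after a short delay destroys itself and decrements the count.
; When none remain, it shows WinScreen, switches to UI-only input with the cursor and pauses the game.
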(event `self.ReceiveBeginPlay`
  (`parent.ReceiveBeginPlay`)
  (bind _asbp_third_person_game_mode (cast `/Game/ThirdPerson/Blueprints/BP_ThirdPersonGameMode` (`GameplayStatics.GetGameMode`)))
  (set `/Game/ThirdPerson/Blueprints/BP_ThirdPersonGameMode.EnemiesLeft` (+ (`/Game/ThirdPerson/Blueprints/BP_ThirdPersonGameMode.EnemiesLeft` _asbp_third_person_game_mode) 1) _asbp_third_person_game_mode))

(event `self.ReceiveAnyDamage`
  (params (Damage :type "Float (single-precision)") (DamageType :type "DamageType Object Reference") (InstigatedBy :type "Controller Object Reference") (DamageCauser :type "Actor Object Reference"))
  (bind _returnvalue (`GameplayStatics.GetPlayerController` 0))
  ;[1 1 1] Handle enemies left Objective
  (if (> (`self.AIHealth`) 0.0)
    (set `self.AIHealth` (- (`self.AIHealth`) Damage))
    (`KismetSystemLibrary.PrintString` "damage recieved")
    (if (not (> (`self.AIHealth`) 0.0))
      (`PrimitiveComponent.SetCollisionEnabled` (`self.Mesh`) "QueryAndPhysics" :!label _label)
      (`PrimitiveComponent.SetSimulatePhysics` (`self.Mesh`) true)
      (`KismetSystemLibrary.Delay` 2.0)
      (`self.K2_DestroyActor`)
      (bind _asbp_third_person_game_mode (cast `/Game/ThirdPerson/Blueprints/BP_ThirdPersonGameMode` (`GameplayStatics.GetGameMode`)))
      (bind _output_get (set `/Game/ThirdPerson/Blueprints/BP_ThirdPersonGameMode.EnemiesLeft` (- (`/Game/ThirdPerson/Blueprints/BP_ThirdPersonGameMode.EnemiesLeft` _asbp_third_person_game_mode) 1) _asbp_third_person_game_mode))
      (if (<= _output_get 0)
        (bind _returnvalue_2 (`|CreateWidget` "/Game/Blueprints/GenralBlueprints/UI/winScreen.winScreen_C"))
        (`UserWidget.AddToViewport` _returnvalue_2 0)
        (set `PlayerController.bShowMouseCursor` true _returnvalue)
        (`WidgetBlueprintLibrary.SetInputMode_UIOnlyEx` _returnvalue null)
        (`GameplayStatics.SetGamePaused` true)))
    (else
      (goto _label))))

(fn `UserConstructionScript`
  (`parent.UserConstructionScript`))