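; Melee enemy character that spots the player with PawnSensing, moves to them and attacks with a punch montage.
; Tick halts its movement until a pawn is seen; each sighting then triggers AI MoveTo toward the player.
; Damage is applied after the montage ends, without a further range check.
; Incoming damage lowers health; a hit received at zero or below ragdolls the mesh and destroys the actor after a delay.
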(event `self.ReceiveTick`
  (params (DeltaSeconds :type "Float (single-precision)"))
  (if (not (`self.isPlayerSeen`))
    (`MovementComponent.StopMovementImmediately` (`self.CharacterMovement`))))

(event `self.PawnSensing.OnSeePawn`
  (params (Pawn :type "Pawn Object Reference"))
  (set `self.isPlayerSeen` true)
  (`self.FollowP`))

(event `FollowP`
  (set `self.canAttack` true)
  (if (`self.isPlayerSeen`)
    (`|AIMoveTo` self (0.0 0.0 0.0) (`GameplayStatics.GetPlayerCharacter` 0) 70.0
      (:`OnSuccess`
        (if (`self.canAttack`)
          (set `self.canAttack` false)
          (bind _returnvalue (`self.PlayAnimMontage` "/Game/animations/AI/AM_Punch1.AM_Punch1"))
          (`KismetSystemLibrary.Delay` _returnvalue)
          (set `self.canAttack` true)
          (bind _asbp_third_person_character (cast `/Game/ThirdPerson/Blueprints/BP_ThirdPersonCharacter` (`GameplayStatics.GetPlayerCharacter` 0)))
          (`GameplayStatics.ApplyDamage` _asbp_third_person_character (`self.Damage`) null self))))
    (else
      (set `self.isPlayerSeen` false))))

(event `self.ReceiveAnyDamage`
  (params (Damage :type "Float (single-precision)") (DamageType :type "DamageType Object Reference") (InstigatedBy :type "Controller Object Reference") (DamageCauser :type "Actor Object Reference"))
  (if (> (`self.AIHealth`) 0.0)
    (set `self.AIHealth` (- (`self.AIHealth`) Damage))
    (`KismetSystemLibrary.PrintString` "damage recieved")
    (else
      (`PrimitiveComponent.SetCollisionEnabled` (`self.Mesh`) "QueryAndPhysics")
      (`PrimitiveComponent.SetSimulatePhysics` (`self.Mesh`) true)
      (`KismetSystemLibrary.Delay` 2.0)
      (`self.K2_DestroyActor`))))

(fn `UserConstructionScript`)