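; Melee enemy AI character that spots the player, punches at close range and takes damage.
; PawnSensing latches IsSeen and sets the "playerSpotted" blackboard key, which Tick holds false until then; the reset logic is unconnected.
; Punchdetection overlap plays a punch montage with movement locked, then box-traces between two arrows to apply damage.
; AnyDamage drains AIhealth; a hit arriving after it is depleted triggers ragdoll and delayed destruction.
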(event `self.ReceiveTick`
  (params (DeltaSeconds :type "Float (single-precision)"))
  (if (not (`self.IsSeen?`))
    (`BlackboardComponent.SetValueAsBool` (`AIBlueprintHelperLibrary.GetBlackboard` (`AIBlueprintHelperLibrary.GetAIController` self)) "playerSpotted" false)))

(event `self.punchdetection.OnComponentEndOverlap`
  (params (OverlappedComponent :type "PrimitiveComponent Object Reference") (OtherActor :type "Actor Object Reference") (OtherComp :type "PrimitiveComponent Object Reference") (OtherBodyIndex :type Integer))
  (cast `/Game/ThirdPerson/Blueprints/BP_ThirdPersonCharacter` OtherActor)
  (set `self.Can Attack` false))

(event `self.punchdetection.OnComponentBeginOverlap`
  (params (OverlappedComponent :type "PrimitiveComponent Object Reference") (OtherActor :type "Actor Object Reference") (OtherComp :type "PrimitiveComponent Object Reference") (OtherBodyIndex :type Integer) (bFromSweep :type Boolean) (SweepResult :type "HitResult Structure (by ref)"))
  (cast `/Game/ThirdPerson/Blueprints/BP_ThirdPersonCharacter` OtherActor)
  (set `self.Can Attack` true)
  (if (`self.Can Attack`)
    (set `self.Can Attack` false)
    (bind _returnvalue (`self.PlayAnimMontage` "/Game/animations/AI/AM_Punch1.AM_Punch1"))
    (`CharacterMovementComponent.DisableMovement` (`self.CharacterMovement`))
    (`KismetSystemLibrary.Delay` _returnvalue)
    (`CharacterMovementComponent.SetMovementMode` (`self.CharacterMovement`) "MOVE_Walking" 0)
    (set `self.Can Attack` true)
    (if (not (<= (`self.AIhealth`) 0.0))
      (bind _outhit (`KismetSystemLibrary.BoxTraceSingle` (`SceneComponent.GetSocketLocation` (`self.Start arrow`) "None") (`SceneComponent.GetSocketLocation` (`self.EndArrow`) "None") (50.0 40.0 40.0) (struct) "TraceTypeQuery1"))
      (cast `/Game/ThirdPerson/Blueprints/BP_ThirdPersonCharacter` (`GameplayStatics.GetPlayerCharacter` 0))
      (`GameplayStatics.ApplyDamage` (`.HitActor` (`GameplayStatics.BreakHitResult` _outhit)) (`self.damage`) null self)
      (if (`self.IsSeen?`)
        (`BlackboardComponent.SetValueAsBool` (`AIBlueprintHelperLibrary.GetBlackboard` (`AIBlueprintHelperLibrary.GetAIController` self)) "playerSpotted" true)
        (else
          (`BlackboardComponent.SetValueAsBool` (`AIBlueprintHelperLibrary.GetBlackboard` (`AIBlueprintHelperLibrary.GetAIController` self)) "playerSpotted" false)
          (set `self.Can Attack` false))))))

(event `self.PawnSensing.OnSeePawn`
  (params (Pawn :type "Pawn Object Reference"))
  (set `self.IsSeen?` true)
  (cast `/Game/ThirdPerson/Blueprints/BP_ThirdPersonCharacter` Pawn)
  (`BlackboardComponent.SetValueAsBool` (`AIBlueprintHelperLibrary.GetBlackboard` (`AIBlueprintHelperLibrary.GetAIController` self)) "playerSpotted" true))

(event `self.ReceiveAnyDamage`
  (params (Damage :type "Float (single-precision)") (DamageType :type "DamageType Object Reference") (InstigatedBy :type "Controller Object Reference") (DamageCauser :type "Actor Object Reference"))
  (if (> (`self.AIhealth`) 0.0)
    (set `self.AIhealth` (- (`self.AIhealth`) Damage))
    (`KismetSystemLibrary.PrintString` "damage recieved")
    (else
      (`PrimitiveComponent.SetCollisionEnabled` (`self.Mesh`) "QueryAndPhysics")
      (`PrimitiveComponent.SetSimulatePhysics` (`self.Mesh`) true)
      (`KismetSystemLibrary.Delay` 2.0)
      (`self.K2_DestroyActor`))))

(fn `UserConstructionScript`)